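; BP_Telephone is an interactable telephone that responds to the first-person character's use-item input with debug messages, escalating to a scare line.
; Its Box overlap binds a handler to the character's OnUseItem dispatcher on entry and unbinds it on exit, so it only responds in range.
; Each use increments InteractedTimes, and a switch on the count prints a repeated greeting, then "Boo!", with no response beyond that.
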(event OnComponentBeginOverlap(Box)
  (params (OverlappedComponent :type Primitive%20Component%20Object%20Reference) (OtherActor :type Actor%20Object%20Reference) (OtherComp :type Primitive%20Component%20Object%20Reference) (OtherBodyIndex :type Integer) (bFromSweep :type Boolean) (SweepResult :type Hit%20Result%20Structure%20%28by%20ref%29))
  (bind _asbp_first_person_character (Utilities|Casting|CastToBP_FirstPersonCharacter OtherActor))
  (EventDispatchers|AssignOnUseItem _asbp_first_person_character (delegate Custom|OnUseItem_Event_0)))

(event OnComponentEndOverlap(Box)
  (params (OverlappedComponent :type Primitive%20Component%20Object%20Reference) (OtherActor :type Actor%20Object%20Reference) (OtherComp :type Primitive%20Component%20Object%20Reference) (OtherBodyIndex :type Integer))
  (bind _asbp_first_person_character (Utilities|Casting|CastToBP_FirstPersonCharacter OtherActor))
  (EventDispatchers|UnbindEventfromOnUseItem _asbp_first_person_character (delegate Custom|OnUseItem_Event_0)))

(event Custom|OnUseItem_Event_0
  (bind _result (Math|Integer|IncrementInt (Variables|Default|GetInteractedTimes))
    (:%20%20
      (switch int _result
        (:1
          (Development|PrintString "Hello" :!label _label))
        (:2
          (goto _label))
        (:3
          (goto _label))
        (:4
          (Development|PrintString "Boo!"))))))

(fn ConstructionScript)