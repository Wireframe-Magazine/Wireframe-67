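; BP_Ghost is an actor that trails the player character, staying directly behind it.
; Every tick it moves itself 100 units along the reverse of player 0's forward vector from that character's location and copies the character's rotation.
; The placement is a hard snap with no interpolation, and the construction script is empty.
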(event EventTick
  (params (DeltaSeconds :type Float%20%28single-precision%29))
  (Transformation|SetActorLocationAndRotation (+ (* (* (Transformation|GetActorForwardVector (Game|GetPlayerCharacter 0)) (Math|Float|MakeLiteralFloat -1.0)) (Math|Float|MakeLiteralFloat 1e+02)) (Transformation|GetActorLocation (Game|GetPlayerCharacter 0))) (Transformation|GetActorRotation (Game|GetPlayerCharacter 0))))

(fn ConstructionScript)