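; Ghost actor that destroys itself once the player has seen it and then loses sight of it.
; Each Tick projects its location to screen space and traces on Visibility from its Arrow component to the player camera.
; An on-screen, unobstructed view resets a start-closed DoOnce, so the next off-screen or blocked frame passes through it to DestroyActor.
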(event EventTick
  (params (DeltaSeconds :type Float%20%28single-precision%29))
  (bind _returnvalue (Game|GetPlayerController 0))
  (bind _returnvalue_2 (Transformation|GetActorLocation))
  (bind _returnvalue_3 (Viewport|GetViewportSize))
  (bind _screenlocation (Class|PlayerController|ProjectWorldLocationtoScreen _returnvalue _returnvalue_2 false))
  (bind (_x _y) (Math|Vector2D|BreakVector2D _screenlocation))
  (bind _returnvalue_4 (Collision|LineTraceByChannel (Transformation|GetWorldLocation (Variables|Default|GetArrow)) (Transformation|GetActorLocation (Game|GetPlayerCameraManager 0)) "TraceTypeQuery1" true 0 "ForDuration"))
  (if (Math|Boolean|ANDBoolean (Math|Float|InRange(Float) _x 0.0 (.x _returnvalue_3)) (Math|Float|InRange(Float) _y 0.0 (.y _returnvalue_3)) (not _returnvalue_4))
    (goto _label Reset)
    (else
      (Utilities|FlowControl|DoOnce true :!label _label
        (:Completed
          (Actor|DestroyActor))))))

(fn ConstructionScript)